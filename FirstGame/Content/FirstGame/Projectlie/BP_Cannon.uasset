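; BP_Cannon is a cannon actor that fires Bullet actors at a fixed interval.
; DoShoot spawns a Bullet at the world location and rotation of its Arrow component.
; ToggleShoot starts or clears a looping timer by function name that calls DoShoot.
; BeginPlay applies the initial Toggle value, and pressing F flips it to switch firing on or off.
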(event EventBeginPlay
  (CallFunction|ToggleShoot (Variables|Default|GetToggle)))

(event EventPressF
  (bind _output_get (Variables|Default|SetToggle (not (Variables|Default|GetToggle))))
  (CallFunction|ToggleShoot _output_get))

(fn ConstructionScript)

(fn DoShoot
  (bind _arrow (Variables|Default|GetArrow))
  (bind _returnvalue (Transformation|GetWorldTransform _arrow))
  (Game|SpawnActorfromClass (Variables|Default|GetBullet) (Math|Transform|MakeTransform (.location _returnvalue) (.rotation _returnvalue) "1.000000,1.000000,1.000000") "Undefined" "MultiplyWithRoot" 0 0))

(fn ToggleShoot
  (params (Toggle :type Boolean))
  (if Toggle
    (Utilities|Time|SetTimerbyFunctionName 0 "DoShoot" 1.0 true)
    (else
      (Utilities|Time|ClearTimerbyFunctionName 0 "DoShoot"))))