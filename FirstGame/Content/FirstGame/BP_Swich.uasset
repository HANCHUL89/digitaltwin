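; BP_Swich is a switch actor that triggers spawning when something overlaps its Cube component.
; On begin overlap it prints the names of the components and actor involved, then calls DoSpawn on its Abc reference.
; End overlap only prints a debug message.
; The construction script sets a TextRender label to the actor's own display name.
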(event OnComponentBeginOverlap(Cube)
  (params (OverlappedComponent :type Primitive%20Component%20Object%20Reference) (OtherActor :type Actor%20Object%20Reference) (OtherComp :type Primitive%20Component%20Object%20Reference) (OtherBodyIndex :type Integer) (bFromSweep :type Boolean) (SweepResult :type Hit%20Result%20Structure%20%28by%20ref%29))
  (Development|PrintString (Utilities|String|Append "Begin Overlap :" "Overlapped Component :" (Utilities|GetDisplayName OverlappedComponent) ", Other Actor :" (Utilities|GetDisplayName OtherActor) ". Other Comp :" (Utilities|GetDisplayName OtherComp)))
  (Default|DoSpawn (Variables|Default|Getabc)))

(event OnComponentEndOverlap(Cube)
  (params (OverlappedComponent :type Primitive%20Component%20Object%20Reference) (OtherActor :type Actor%20Object%20Reference) (OtherComp :type Primitive%20Component%20Object%20Reference) (OtherBodyIndex :type Integer))
  (Development|PrintString "End Over Lap"))

(fn ConstructionScript
  (Rendering|Components|TextRender|SetText (Variables|Default|GetTextRender) (Utilities|Text|ToText(String) (Utilities|GetDisplayName self))))