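; Blueprint that moves its Cube component around a square path in the local X-Z plane.
; Each Tick switches on the MoveType2 state, steps one coordinate by a fixed amount and sets the Cube's relative location.
; Reaching a bound (0 or 1000) advances the state in an up, right, down, left loop.
; Steps ignore delta time, so speed depends on frame rate.
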(event EventTick
  (params (DeltaSeconds :type Float%20%28single-precision%29))
  (switch Utilities|FlowControl|Switch|SwitchonENUM_MoveType2 (Variables|Default|GetMoveType2)
    (:NewEnumerator0
      (bind _output_get (Variables|Default|SetZ의%20위치 (+ (Variables|Default|GetZ의%20위치) 1e+01)))
      (Transformation|SetRelativeLocation (Variables|Default|GetCube) (Math|Vector|MakeVector (Variables|Default|GetX의%20위치) 0.0 _output_get) false false)
      (if (>= (Variables|Default|GetZ의%20위치) 1e+03)
        (Variables|Default|SetMoveType2 "NewEnumerator1")))
    (:NewEnumerator1
      (bind _output_get_2 (Variables|Default|SetX의%20위치 (+ (Variables|Default|GetX의%20위치) 1e+01)))
      (Transformation|SetRelativeLocation (Variables|Default|GetCube) (Math|Vector|MakeVector _output_get_2 0.0 (Variables|Default|GetZ의%20위치)) false false)
      (if (>= (Variables|Default|GetX의%20위치) 1e+03)
        (Variables|Default|SetMoveType2 "NewEnumerator2")))
    (:NewEnumerator2
      (bind _output_get_3 (Variables|Default|SetZ의%20위치 (+ (Variables|Default|GetZ의%20위치) -1e+01)))
      (Transformation|SetRelativeLocation (Variables|Default|GetCube) (Math|Vector|MakeVector (Variables|Default|GetX의%20위치) 0.0 _output_get_3) false false)
      (if (<= (Variables|Default|GetZ의%20위치) 0.0)
        (Variables|Default|SetMoveType2 "NewEnumerator3")))
    (:NewEnumerator3
      (bind _output_get_4 (Variables|Default|SetX의%20위치 (+ (Variables|Default|GetX의%20위치) -1e+01)))
      (Transformation|SetRelativeLocation (Variables|Default|GetCube) (Math|Vector|MakeVector _output_get_4 0.0 (Variables|Default|GetZ의%20위치)) false false)
      (if (<= (Variables|Default|GetX의%20위치) 0.0)
        (Variables|Default|SetMoveType2 "NewEnumerator0")))))

(fn ConstructionScript)