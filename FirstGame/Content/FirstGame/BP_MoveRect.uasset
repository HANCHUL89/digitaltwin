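; Actor that moves its Cube component endlessly around a square path in the local X-Z plane.
; Each tick, a switch on the MoveType state steps the X or Z position by a fixed amount and applies it as the relative location.
; Reaching a boundary advances the state through Right, Up, Left and Down.
; The step ignores delta time, so speed depends on frame rate.
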(event EventTick
  (params (DeltaSeconds :type Float%20%28single-precision%29))
  (switch Utilities|FlowControl|Switch|SwitchonENUM_Move (Variables|Default|GetMoveType)
    (:NewEnumerator0
      (bind _output_get (Variables|Default|SetX의%20위치 (+ (Variables|Default|GetX의%20위치) 1e+01)))
      (Transformation|SetRelativeLocation (Variables|Default|GetCube) (Math|Vector|MakeVector _output_get 0.0 (Variables|Default|GetZ의%20위치)) false false)
      ;[0.15 0.15 0.15 0.5] If
      (if (>= (Variables|Default|GetX의%20위치) 5e+02)
        (Variables|Default|SetMoveType "NewEnumerator1")))
    (:NewEnumerator1
      (bind _output_get_2 (Variables|Default|SetZ의%20위치 (+ (Variables|Default|GetZ의%20위치) 1e+01)))
      (Transformation|SetRelativeLocation (Variables|Default|GetCube) (Math|Vector|MakeVector (Variables|Default|GetX의%20위치) 0.0 _output_get_2) false false)
      ;[0.15 0.15 0.15 0.5] If
      (if (>= (Variables|Default|GetZ의%20위치) 5e+02)
        (Variables|Default|SetMoveType "NewEnumerator2")))
    (:NewEnumerator2
      (Variables|Default|SetX의%20위치 (+ (Variables|Default|GetX의%20위치) -1e+01))
      (Transformation|SetRelativeLocation (Variables|Default|GetCube) (Math|Vector|MakeVector (Variables|Default|GetX의%20위치) 0.0 (Variables|Default|GetZ의%20위치)) false false)
      ;[0.15 0.15 0.15 0.5] If
      (if (<= (Variables|Default|GetX의%20위치) 0.0)
        (Variables|Default|SetMoveType "NewEnumerator3")))
    (:NewEnumerator3
      (Variables|Default|SetZ의%20위치 (+ (Variables|Default|GetZ의%20위치) -1e+01))
      (Transformation|SetRelativeLocation (Variables|Default|GetCube) (Math|Vector|MakeVector (Variables|Default|GetX의%20위치) 0.0 (Variables|Default|GetZ의%20위치)) false false)
      ;[0.15 0.15 0.15 0.5] If
      (if (<= (Variables|Default|GetZ의%20위치) 0.0)
        (Variables|Default|SetMoveType "NewEnumerator0")))))

(fn ConstructionScript)