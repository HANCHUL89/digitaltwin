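; BP_Counter is a counter with a Widget component that displays a number cycling from 0 to 9.
; Its PressF event increments Count through UpdateCount, which wraps to 0 after 9, then passes the value to the component's CountWidget.
; Tick rotates the widget to face the player camera.
; Older count-down and text-setting logic remains in the graph but never runs.
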(event EventPressF
  (CallFunction|UpdateCount)
  (bind _ascount_widget (Utilities|Casting|CastToCountWidget (UserInterface|GetUserWidgetObject (Variables|Default|GetWidget))))
  (Default|UpdateCount _ascount_widget (Variables|Default|GetCount)))

(event EventTick
  (params (DeltaSeconds :type Float%20%28single-precision%29))
  (Transformation|SetWorldRotation (Variables|Default|GetWidget) (Math|Rotator|FindLookatRotation (Transformation|GetWorldLocation (Variables|Default|GetWidget)) (Transformation|GetActorLocation (Game|GetPlayerCameraManager 0))) false false))

(fn ConstructionScript)

(fn UpdateCount
  ;[0.15 0.15 0.15 0.5] Count값이 1씩 증가
  (Variables|Default|SetCount (+ (Variables|Default|GetCount) 1))
  ;[0.15 0.15 0.15 0.5] 만약에 Count가 9보다 크면 0으로 변경
  (if (> (Variables|Default|GetCount) 9)
    (Variables|Default|SetCount 0)))