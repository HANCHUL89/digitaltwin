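; BP_Switch is a toggleable switch with a floating name label.
; Its PressF event flips IsSwitchOn and calls SwitchOn or SwitchOff to match the new state.
; The construction script sets the TextRender label to the object's display name, and Tick rotates the label each frame to face the player camera.
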(event EventPressF
  (bind _output_get (Variables|Default|SetIsSwitchOn (not (Variables|Default|GetIsSwitchOn))))
  (if _output_get
    (CallFunction|Switchon)
    (else
      (CallFunction|SwitchOff))))

(event EventTick
  (params (DeltaSeconds :type Float%20%28single-precision%29))
  (Transformation|SetWorldRotation (Variables|Default|GetTextRender) (Math|Rotator|FindLookatRotation (Transformation|GetWorldLocation (Variables|Default|GetTextRender)) (Transformation|GetActorLocation (Game|GetPlayerCameraManager 0))) false false))

(fn ConstructionScript
  (Rendering|Components|TextRender|SetText (Variables|Default|GetTextRender) (Utilities|Text|ToText(String) (Utilities|GetDisplayName self))))