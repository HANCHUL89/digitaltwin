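; BP_SplineMove is an actor that moves a cube back and forth along its spline from BeginPlay.
; A timeline value, scaled by spline length, gives the distance sampled on each update to position the cube.
; When the timeline finishes, it flips IsRight and plays or reverses, forming an endless ping-pong.
; The spline point is read in local space but applied as a world location.
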(event EventBeginPlay
  (bind _spline (Variables|Default|GetSpline))
  (if (Variables|Default|GetIs%20Right) :!label _label
    (bind _value (Timeline|타임라인 Play)
      (:Update
        (Transformation|SetWorldLocation (Variables|Default|GetCube) (.location (Spline|GetTransformatDistanceAlongSpline _spline (* _value (Spline|GetSplineLength _spline)) "Local" false)) false false))
      (:Finished
        (Variables|Default|SetIs%20Right (not (Variables|Default|GetIs%20Right)))
        (goto _label)))
    (else
      (Timeline|타임라인 Reverse))))

(fn ConstructionScript)