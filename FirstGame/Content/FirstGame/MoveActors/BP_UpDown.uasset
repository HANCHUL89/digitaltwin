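; BP_UpDown is a moving actor whose Cone bounces up and down along relative Z while play is enabled.
; Tick steps the height by a fixed, frame-rate-dependent amount and flips direction at the upper and lower limits.
; BeginPlay binds to a Switch's toggle dispatcher, and EventSwitchToggle sets the IsPlay flag from the toggle value to start or pause the motion.
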(event EventBeginPlay
  (EventDispatchers|BindEventtoNewEventDispatcherToggleSwitch (Variables|Default|GetSwitch) (EventDispatchers|CreateEvent :!event EventSwitchToggle)))

(event EventTick
  (params (DeltaSeconds :type Float%20%28single-precision%29))
  (if (Variables|Default|GetIsPlay)
    (if (Variables|Default|GetIsMoveUp)
      (Variables|Default|SetLocz (+ (Variables|Default|GetLocz) 1e+01))
      (Transformation|SetRelativeLocation (Variables|Default|GetCone) (Math|Vector|MakeVector 0.0 0.0 (Variables|Default|GetLocz)) false false)
      ;[0.15 0.15 0.15 0.5] If
      (if (>= (Variables|Default|GetLocz) 5e+02)
        (Variables|Default|SetIsMoveUp false))
      (else
        (Variables|Default|SetLocz (+ (Variables|Default|GetLocz) -1e+01))
        (Transformation|SetRelativeLocation (Variables|Default|GetCone) (Math|Vector|MakeVector 0.0 0.0 (Variables|Default|GetLocz)) false false)
        ;[0.15 0.15 0.15 0.5] If
        (if (<= (Variables|Default|GetLocz) 0.0)
          (Variables|Default|SetIsMoveUp true))))))

(fn ConstructionScript)

(fn EventSwitchToggle
  (params (Toggle :type Boolean))
  (Variables|Default|SetIsPlay Toggle))

(fn DoPlayandStop
  (params (IsPlay :type Boolean))
  (Variables|Default|SetIsPlay IsPlay)
  (return false))