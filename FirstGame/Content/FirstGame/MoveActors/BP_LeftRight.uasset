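; BP_LeftRight is an actor whose Box slides back and forth along relative X between two fixed limits while IsPlay is true.
; Each Tick steps the position by a fixed amount without delta-time scaling, flipping a direction flag at either limit.
; On BeginPlay it binds to the UpdateSwitch dispatcher of every actor in the Switch array.
; EventUpdateSwitch and DoPlayAndStop both set IsPlay to start or stop movement.
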(event OnComponentHit(Box)
  (params (HitComponent :type Primitive%20Component%20Object%20Reference) (OtherActor :type Actor%20Object%20Reference) (OtherComp :type Primitive%20Component%20Object%20Reference) (NormalImpulse :type Vector :default "0, 0, 0") (Hit :type Hit%20Result%20Structure%20%28by%20ref%29)))

(event EventTick
  (params (DeltaSeconds :type Float%20%28single-precision%29))
  (if (Variables|Default|GetIsPlay)
    (if (Variables|Default|Get오른쪽%20이동인가?)
      (CallFunction|오른쪽으로10만큼이동)
      ;[0.15 0.15 0.15 0.5] If
      (if (>= (Variables|Default|GetX의%20위치) 5e+02)
        (Variables|Default|Set오른쪽%20이동인가? false))
      (else
        (CallFunction|왼쪽으로10만큼이동)
        ;[0.15 0.15 0.15 0.5] If
        (if (<= (Variables|Default|GetX의%20위치) 0.0)
          (Variables|Default|Set오른쪽%20이동인가? true))))))

(event EventBeginPlay
  (for _array_element (Variables|Default|GetSwitch)
    (EventDispatchers|BindEventtoEventDispatcherUpdateSwitch _array_element (EventDispatchers|CreateEvent :!event EventUpdateSwitch))))

(fn ConstructionScript)

(fn 오른쪽으로10만큼이동
  ;[0.15 0.15 0.15 0.5] 오른쪽으로 이동한다.
  ;;[0.15 0.15 0.15 0.5] X의 위치에 100을 더한다
  (Variables|Default|SetX의%20위치 (+ (Variables|Default|GetX의%20위치) 1e+01))
  ;;[0.15 0.15 0.15 0.5] Box의 상대좌표 X를 "X의 위치"값으로 변경한다
  (Transformation|SetRelativeLocation (Variables|Default|GetBox) (Math|Vector|MakeVector (Variables|Default|GetX의%20위치) 0.0 0.0) false false))

(fn 왼쪽으로10만큼이동
  ;[0.15 0.15 0.15 0.5] 왼쪽으로 이동한다.
  ;;[0.15 0.15 0.15 0.5] X의 위치에 100을 더한다
  (Variables|Default|SetX의%20위치 (+ (Variables|Default|GetX의%20위치) -1e+01))
  ;;[0.15 0.15 0.15 0.5] Box의 상대좌표 X를 "X의 위치"값으로 변경한다
  (Transformation|SetRelativeLocation (Variables|Default|GetBox) (Math|Vector|MakeVector (Variables|Default|GetX의%20위치) 0.0 0.0) false false))

(fn EventUpdateSwitch
  (params (IsSwitchOn :type Boolean))
  (Variables|Default|SetIsPlay IsSwitchOn))

(fn DoPlayandStop
  (params (IsPlay :type Boolean))
  (Variables|Default|SetIsPlay IsPlay)
  (return true))