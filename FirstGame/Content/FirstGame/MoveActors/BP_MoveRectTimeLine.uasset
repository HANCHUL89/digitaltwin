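; Actor that moves a Cube along a looping Timeline-driven path, started and stopped by switch actors.
; BeginPlay binds to the update dispatcher of each entry in the Switch array, and EventSwitchToggle maps a toggle to DoPlay or DoStop.
; DoPlay runs only when IsRight is set, scaling the Timeline vector into the Cube's relative location and restarting on finish.
; DoPlayAndStop offers the same play/stop control as a function.
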(event Custom|DoStop
  (bind _vector (Timeline|타임라인 Stop)
    (:Update
      (Transformation|SetRelativeLocation (Variables|Default|GetCube) (* _vector 1e+03) false false))
    (:Finished
      (Timeline|타임라인 PlayFromStart))))

(event Custom|DoPlay
  (if (Variables|Default|GetIsRight)
    (bind _vector (Timeline|타임라인 Play)
      (:Update
        (Transformation|SetRelativeLocation (Variables|Default|GetCube) (* _vector 1e+03) false false))
      (:Finished
        (Timeline|타임라인 PlayFromStart)))))

(event EventBeginPlay
  (for _array_element (Variables|Default|GetSwitch)
    (EventDispatchers|BindEventtoEventDispatcherUpdateSwitch _array_element (EventDispatchers|CreateEvent :!event EventSwitchToggle))))

(fn ConstructionScript)

(fn EventSwitchToggle
  (params (Toggle :type Boolean))
  (if Toggle
    (CallFunction|DoPlay)
    (else
      (CallFunction|DoStop)))
  (return))

(fn DoPlayandStop
  (params (IsPlay :type Boolean))
  (if IsPlay
    (CallFunction|Doplay)
    (else
      (CallFunction|DoStop)))
  (return false))