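; BP_MoveRect is an actor that moves its Cube around a square loop in the local XZ plane while IsPlay is true.
; Tick runs a MoveType state machine (Right, Up, Left, Down), stepping a fixed amount per frame, independent of delta time, and turning at each bound.
; BeginPlay binds to each Switch's update dispatcher.
; EventUpdateSwitch and DoPlayAndStop both set IsPlay to start or stop motion.
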(event EventBeginPlay
  (for _array_element (Variables|Default|GetSwitch)
    (EventDispatchers|BindEventtoEventDispatcherUpdateSwitch _array_element (EventDispatchers|CreateEvent :!event EventUpdateSwitch))))

(event EventTick
  (params (DeltaSeconds :type Float%20%28single-precision%29))
  (if (Variables|Default|GetIsPlay)
    (switch Utilities|FlowControl|Switch|SwitchonENUM_Move (Variables|Default|GetMoveType)
      (:NewEnumerator0
        (CallFunction|오른쪽으로이동)
        ;[0.15 0.15 0.15 0.5] If
        (if (>= (Variables|Default|GetX의%20위치) 5e+02)
          (Variables|Default|SetMoveType "NewEnumerator1")))
      (:NewEnumerator1
        (CallFunction|위쪽으로이동)
        ;[0.15 0.15 0.15 0.5] If
        (if (>= (Variables|Default|GetZ의%20위치) 5e+02)
          (Variables|Default|SetMoveType "NewEnumerator2")))
      (:NewEnumerator2
        (CallFunction|왼쪽으로이동)
        ;[0.15 0.15 0.15 0.5] If
        (if (<= (Variables|Default|GetX의%20위치) 0.0)
          (Variables|Default|SetMoveType "NewEnumerator3")))
      (:NewEnumerator3
        (CallFunction|아래쪽으로이동)
        ;[0.15 0.15 0.15 0.5] If
        (if (<= (Variables|Default|GetZ의%20위치) 0.0)
          (Variables|Default|SetMoveType "NewEnumerator0"))))))

(fn ConstructionScript)

(fn 오른쪽으로이동
  (bind _output_get (Variables|Default|SetX의%20위치 (+ (Variables|Default|GetX의%20위치) 1e+01)))
  (Transformation|SetRelativeLocation (Variables|Default|GetCube) (Math|Vector|MakeVector _output_get 0.0 (Variables|Default|GetZ의%20위치)) false false))

(fn 위쪽으로이동
  (bind _output_get (Variables|Default|SetZ의%20위치 (+ (Variables|Default|GetZ의%20위치) 1e+01)))
  (Transformation|SetRelativeLocation (Variables|Default|GetCube) (Math|Vector|MakeVector (Variables|Default|GetX의%20위치) 0.0 _output_get) false false))

(fn 왼쪽으로이동
  (Variables|Default|SetX의%20위치 (+ (Variables|Default|GetX의%20위치) -1e+01))
  (Transformation|SetRelativeLocation (Variables|Default|GetCube) (Math|Vector|MakeVector (Variables|Default|GetX의%20위치) 0.0 (Variables|Default|GetZ의%20위치)) false false))

(fn 아래쪽으로이동
  (Variables|Default|SetZ의%20위치 (+ (Variables|Default|GetZ의%20위치) -1e+01))
  (Transformation|SetRelativeLocation (Variables|Default|GetCube) (Math|Vector|MakeVector (Variables|Default|GetX의%20위치) 0.0 (Variables|Default|GetZ의%20위치)) false false))

(fn EventUpdateSwitch
  (params (Toggle :type Boolean))
  (Variables|Default|SetIsPlay Toggle))

(fn DoPlayandStop
  (params (IsPlay :type Boolean))
  (Variables|Default|SetIsPlay IsPlay)
  (return false))