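; BP_Spawnr is a spawner Blueprint that creates actors of a configurable class at random points inside its Box component.
; Each DoSpawn event spawns one actor and increments SpawnCount until it reaches a hard cap of five; nothing in this graph triggers the event or resets the count.
; Spawn points use half the box's scaled extent as half-size, so they fall only within the central half of each axis.
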(event Custom|DoSpawn
  (bind _box (Variables|Default|GetBox))
  (if (< (Variables|Default|GetSpawnCount) 5)
    (Game|SpawnActorfromClass (Variables|Default|GetSpawnActorClass) (Math|Transform|MakeTransform (Math|Random|RandomPointinBoundingBox (Transformation|GetWorldLocation _box) (/ (Components|Box|GetScaledBoxExtent _box) 2.0)) "0, 0, 0" "1.000000,1.000000,1.000000") "Undefined" "MultiplyWithRoot" 0 0)
    (Variables|Default|SetSpawnCount (+ (Variables|Default|GetSpawnCount) 1))))

(fn ConstructionScript)