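; BP_ProductionManager runs a production batch, spawning BP_material actors at its SpawnPoint until a requested quantity is reached.
; StartProduction stores the target, resets the count, sets the running flag and starts a looping one-second timer on SpawnOneMaterial.
; Each tick spawns one material, increments the count and broadcasts OnQtyChanged, then clears the timer once the target is met.
; The running flag is not reset on completion.
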(event Custom|StartProduction
  (params (InTargetQty :type Integer))
  (Variables|Default|SetTargetQty InTargetQty)
  (Variables|Default|SetCurrentQty 0)
  (Variables|Default|SetBIsRunning true)
  (Development|PrintString "생산시작 - 목표수량 :")
  (bind _returnvalue (Utilities|Time|SetTimerbyFunctionName 0 "SpawnOneMaterial" 1.0 true))
  (Variables|Default|SetSpawnTimerHandle _returnvalue))

(event Custom|SpawnOneMaterial
  (Game|SpawnActorfromClass "/Game/FactoryProject/BP/BP_material.BP_material_C" (Transformation|GetWorldTransform (Variables|Default|GetSpawnPoint)) "Undefined" "MultiplyWithRoot" 0 0)
  (bind _output_get (Variables|Default|SetCurrentQty (+ (Variables|Default|GetCurrentQty) 1)))
  (Default|CallOnQtyChanged _output_get)
  (if (>= (Variables|Default|GetCurrentQty) (Variables|Default|GetTargetQty))
    (Utilities|Time|ClearandInvalidateTimerbyHandle (Variables|Default|GetSpawnTimerHandle))
    (Development|PrintString "Timer")))

(fn ConstructionScript)