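; BP_Belt is a conveyor belt actor that pushes BP_Box actors along the world X axis.
; Every tick it queries its Box trigger for overlapping BP_Box actors and sets a fixed linear velocity on the Cube of a BPBox reference, replacing current velocity.
; The overlap event is empty, and an older impulse-based push with a debug print is left disconnected.
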(event OnComponentBeginOverlap(Box)
  (params (OverlappedComponent :type Primitive%20Component%20Object%20Reference) (OtherActor :type Actor%20Object%20Reference) (OtherComp :type Primitive%20Component%20Object%20Reference) (OtherBodyIndex :type Integer) (bFromSweep :type Boolean) (SweepResult :type Hit%20Result%20Structure%20%28by%20ref%29)))

(event EventTick
  (params (DeltaSeconds :type Float%20%28single-precision%29))
  (for _array_element (Collision|GetOverlappingActors (Variables|Default|GetBox) "/Game/FirstProject/BP_Box.BP_Box_C" :!class /Script/Engine.PrimitiveComponent)
    (Physics|SetPhysicsLinearVelocity (Variables|/Game/FirstProject/BP_Box.BP_Box_C|GetCube (Variables|Default|GetBP_Box)) "10.000000,0.000000,0.000000" false "None")))

(fn ConstructionScript)