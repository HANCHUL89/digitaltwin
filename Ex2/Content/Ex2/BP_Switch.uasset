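; BP_Switch is a switch that starts and stops a set of actors through the BPI_PlayAndStop interface.
; Each PressF event flips a Toggle flag, then loops over the Actors array, casts each entry to the interface and calls DoPlayAndStop with the new state.
; The switch also has its own DoPlayAndStop function, which is left empty.
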(event EventPressF
  (bind _output_get (Variables|Default|Settoggle (not (Variables|Default|Gettoggle))))
  (if _output_get
    (for _array_element (Variables|Default|GetActors)
      (bind _asbpi_play_and_stop (Utilities|Casting|CastToBPI_PlayAndStop _array_element))
      (Default|DoPlayandStop _asbpi_play_and_stop true))
    (else
      (for _array_element_2 (Variables|Default|GetActors)
        (bind _asbpi_play_and_stop_2 (Utilities|Casting|CastToBPI_PlayAndStop _array_element_2))
        (Default|DoPlayandStop _asbpi_play_and_stop_2 false)))))

(fn ConstructionScript)

(fn DoPlayandStop
  (params (Isplay :type Boolean)))