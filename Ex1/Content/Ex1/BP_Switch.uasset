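; BP_Switch is a trigger switch that runs a list of target actors while its Cube is overlapped and stops them when an overlap ends.
; Each overlap event loops over Actors and casts through BP_LeftRight, BP_LeftRightTimeLine, BP_MoveRect and BP_Timer.
; The timeline variant gets DoPlay or DoStop calls, while the others have IsPlay toggled.
; Tick rotates the TextRender label to face the player camera.
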(event OnComponentBeginOverlap(Cube)
  (params (OverlappedComponent :type Primitive%20Component%20Object%20Reference) (OtherActor :type Actor%20Object%20Reference) (OtherComp :type Primitive%20Component%20Object%20Reference) (OtherBodyIndex :type Integer) (bFromSweep :type Boolean) (SweepResult :type Hit%20Result%20Structure%20%28by%20ref%29))
  (for _array_element (Variables|Default|GetActors)
    (bind _asbp_left_right (Utilities|Casting|CastToBP_LeftRight _array_element)
      (:then
        (Variables|/Game/Ex1/BP_LeftRight.BP_LeftRight_C|SetIsPlay _asbp_left_right true))
      (:CastFailed
        (bind _asbp_left_right_time_line (Utilities|Casting|CastToBP_LeftRightTimeLine _array_element)
          (:then
            (Default|DoPlay _asbp_left_right_time_line))
          (:CastFailed
            (bind _asbp_move_rect (Utilities|Casting|CastToBP_MoveRect _array_element)
              (:then
                (Variables|/Game/Ex1/BP_MoveRect.BP_MoveRect_C|SetIsPlay _asbp_move_rect true))
              (:CastFailed
                (bind _asbp_timer (Utilities|Casting|CastToBP_Timer _array_element))
                (Variables|/Game/Ex1/BP_Timer.BP_Timer_C|SetIsPlay _asbp_timer true)))))))))

(event OnComponentEndOverlap(Cube)
  (params (OverlappedComponent :type Primitive%20Component%20Object%20Reference) (OtherActor :type Actor%20Object%20Reference) (OtherComp :type Primitive%20Component%20Object%20Reference) (OtherBodyIndex :type Integer))
  (for _array_element (Variables|Default|GetActors)
    (bind _asbp_left_right (Utilities|Casting|CastToBP_LeftRight _array_element)
      (:then
        (Variables|/Game/Ex1/BP_LeftRight.BP_LeftRight_C|SetIsPlay _asbp_left_right false))
      (:CastFailed
        (bind _asbp_left_right_time_line (Utilities|Casting|CastToBP_LeftRightTimeLine _array_element)
          (:then
            (Default|DoStop _asbp_left_right_time_line))
          (:CastFailed
            (bind _asbp_move_rect (Utilities|Casting|CastToBP_MoveRect _array_element)
              (:then
                (Variables|/Game/Ex1/BP_MoveRect.BP_MoveRect_C|SetIsPlay _asbp_move_rect false))
              (:CastFailed
                (bind _asbp_timer (Utilities|Casting|CastToBP_Timer _array_element))
                (Variables|/Game/Ex1/BP_Timer.BP_Timer_C|SetIsPlay _asbp_timer false)))))))))

(event EventTick
  (params (DeltaSeconds :type Float%20%28single-precision%29))
  (Transformation|SetWorldRotation (Variables|Default|GetTextRender) (Math|Rotator|FindLookatRotation (Transformation|GetWorldLocation (Variables|Default|GetTextRender)) (Transformation|GetActorLocation (Game|GetPlayerCameraManager 0))) false false))

(fn ConstructionScript)