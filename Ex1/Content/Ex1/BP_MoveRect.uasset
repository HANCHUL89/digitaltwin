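; Exercise Blueprint that moves its Cube component around a square path in the XZ plane while IsPlay is true.
; Each Tick, a switch on MoveType steps the stored X or Z position by a fixed amount and applies it as the cube's relative location.
; Reaching a corner switches MoveType to the next direction, looping Right, Up, Left, Down.
; Movement is per frame without delta time scaling, so speed depends on frame rate.
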(event EventTick
  (params (DeltaSeconds :type Float%20%28single-precision%29))
  (if (Variables|Default|GetIsPlay)
    (switch Utilities|FlowControl|Switch|SwitchonENUM_MoveRect (Variables|Default|GetMoveType)
      (:NewEnumerator0
        (bind _output_get (Variables|Default|SetX의%20위치 (+ (Variables|Default|GetX의%20위치) 1e+01)))
        (Transformation|SetRelativeLocation (Variables|Default|GetCube) (Math|Vector|MakeVector _output_get 0.0 (Variables|Default|GetZ의%20위치)) false false)
        (if (>= (Variables|Default|GetX의%20위치) 5e+02)
          (Variables|Default|SetMoveType "NewEnumerator1")))
      (:NewEnumerator1
        (bind _output_get_2 (Variables|Default|SetZ의%20위치 (+ (Variables|Default|GetZ의%20위치) 1e+01)))
        (Transformation|SetRelativeLocation (Variables|Default|GetCube) (Math|Vector|MakeVector (Variables|Default|GetX의%20위치) 0.0 _output_get_2) false false)
        (if (>= (Variables|Default|GetZ의%20위치) 5e+02)
          (Variables|Default|SetMoveType "NewEnumerator2")))
      (:NewEnumerator2
        (bind _output_get_3 (Variables|Default|SetX의%20위치 (+ (Variables|Default|GetX의%20위치) -1e+01)))
        (Transformation|SetRelativeLocation (Variables|Default|GetCube) (Math|Vector|MakeVector _output_get_3 0.0 (Variables|Default|GetZ의%20위치)) false false)
        (if (<= (Variables|Default|GetX의%20위치) 0.0)
          (Variables|Default|SetMoveType "NewEnumerator3")))
      (:NewEnumerator3
        (bind _output_get_4 (Variables|Default|SetZ의%20위치 (+ (Variables|Default|GetZ의%20위치) -1e+01)))
        (Transformation|SetRelativeLocation (Variables|Default|GetCube) (Math|Vector|MakeVector (Variables|Default|GetX의%20위치) 0.0 _output_get_4) false false)
        (if (<= (Variables|Default|GetZ의%20위치) 0.0)
          (Variables|Default|SetMoveType "NewEnumerator0"))))))

(fn ConstructionScript)