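; BP_LeftRight is an actor that slides its Cube component back and forth along the relative X axis while IsPlay is true.
; Each Tick steps the stored X position (X의위치) by a fixed amount and applies it to the Cube.
; A direction flag (오른쪽이동인가, "is moving right") flips at either bound of the range.
; The step ignores delta time, so speed depends on frame rate.
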(event EventTick
  (params (DeltaSeconds :type Float%20%28single-precision%29))
  (if (Variables|Default|GetIsPlay)
    (if (Variables|Default|Get오른쪽이동인가?)
      ;[0.15 0.15 0.15 0.5] X의 위치가 10씩 증가
      (bind _output_get (Variables|Default|SetX의%20위치 (+ (Variables|Default|GetX의%20위치) 1e+01)))
      (Transformation|SetRelativeLocation (Variables|Default|GetCube) (Math|Vector|MakeVector _output_get 0.0 0.0) false false)
      (if (>= (Variables|Default|GetX의%20위치) 5e+02)
        (Variables|Default|Set오른쪽이동인가? false))
      (else
        ;[0.15 0.15 0.15 0.5] X의 위치가 10씩 증가
        (Variables|Default|SetX의%20위치 (+ (Variables|Default|GetX의%20위치) -1e+01))
        (Transformation|SetRelativeLocation (Variables|Default|GetCube) (Math|Vector|MakeVector (Variables|Default|GetX의%20위치) 0.0 0.0) false false)
        (if (<= (Variables|Default|GetX의%20위치) 0.0)
          (Variables|Default|Set오른쪽이동인가? true))))))

(fn ConstructionScript)