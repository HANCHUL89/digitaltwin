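; BP_CountBox is a collect-game actor that keeps a count and shows it on a widget component.
; Two custom events raise or lower Count by one and pass it to CountWidget's UpdateCount.
; Tick rotates the widget to face the player camera.
; The separate AddCount function only prints a debug string and leaves Count unchanged.
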(event Custom|커스텀이벤트
  ;[0.15 0.15 0.15 0.5] Count가 1씩 증가
  (Variables|Default|SetCount (+ (Variables|Default|GetCount) 1))
  (bind _ascount_widget (Utilities|Casting|CastToCountWidget (UserInterface|GetUserWidgetObject (Variables|Default|GetWidget))))
  (Default|UpdateCount _ascount_widget (Variables|Default|GetCount)))

(event Custom|커스텀이벤트_0
  ;[0.15 0.15 0.15 0.5] Count가 1씩 감소
  (Variables|Default|SetCount (+ (Variables|Default|GetCount) -1))
  ;[0.15 0.15 0.15 0.5] 표시한다
  (bind _ascount_widget (Utilities|Casting|CastToCountWidget (UserInterface|GetUserWidgetObject (Variables|Default|GetWidget))))
  (Default|UpdateCount _ascount_widget (Variables|Default|GetCount)))

(event EventTick
  (params (DeltaSeconds :type Float%20%28single-precision%29))
  (Transformation|SetWorldRotation (Variables|Default|GetWidget) (Math|Rotator|FindLookatRotation (Transformation|GetWorldLocation (Variables|Default|GetWidget)) (Transformation|GetActorLocation (Game|GetPlayerCameraManager 0))) false false))

(fn ConstructionScript)

(fn AddCount
  (Development|PrintString "AddCount"))