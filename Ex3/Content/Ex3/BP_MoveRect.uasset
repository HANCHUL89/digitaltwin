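; Exercise actor that moves its Cube around a 500-unit square in the relative X-Z plane while IsPlay is set.
; Tick switches on the MoveRect state (Right, Up, Left, Down), calling ±10 step functions and changing state at each corner.
; Steps are fixed per frame with no delta time, so speed follows frame rate.
; DoPlayAndStop sets IsPlay to start or pause the motion.
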(event EventTick
  (params (DeltaSeconds :type Float%20%28single-precision%29))
  (if (Variables|Default|GetIsPlay)
    (switch Utilities|FlowControl|Switch|SwitchonENUM_MoveRect (Variables|Default|GetMoveRect)
      (:NewEnumerator0
        (CallFunction|X의위치가+10)
        (if (>= (Variables|Default|GetX의%20위치) 5e+02)
          (Variables|Default|SetMoveRect "NewEnumerator1")))
      (:NewEnumerator1
        (CallFunction|Z의위치가+10)
        (if (>= (Variables|Default|GetZ의%20위치) 5e+02)
          (Variables|Default|SetMoveRect "NewEnumerator2")))
      (:NewEnumerator2
        (CallFunction|X의위치가-10)
        (if (<= (Variables|Default|GetX의%20위치) 0.0)
          (Variables|Default|SetMoveRect "NewEnumerator3")))
      (:NewEnumerator3
        (CallFunction|Z의위치가-10)
        (if (<= (Variables|Default|GetZ의%20위치) 0.0)
          (Variables|Default|SetMoveRect "NewEnumerator0"))))))

(fn ConstructionScript)

(fn X의위치가+10
  (bind _output_get (Variables|Default|SetX의%20위치 (+ (Variables|Default|GetX의%20위치) 1e+01)))
  (Transformation|SetRelativeLocation (Variables|Default|GetCube) (Math|Vector|MakeVector _output_get 0.0 (Variables|Default|GetZ의%20위치)) false false))

(fn Z의위치가+10
  (bind _output_get (Variables|Default|SetZ의%20위치 (+ (Variables|Default|GetZ의%20위치) 1e+01)))
  (Transformation|SetRelativeLocation (Variables|Default|GetCube) (Math|Vector|MakeVector (Variables|Default|GetX의%20위치) 0.0 _output_get) false false))

(fn X의위치가-10
  (bind _output_get (Variables|Default|SetX의%20위치 (+ (Variables|Default|GetX의%20위치) -1e+01)))
  (Transformation|SetRelativeLocation (Variables|Default|GetCube) (Math|Vector|MakeVector _output_get 0.0 (Variables|Default|GetZ의%20위치)) false false))

(fn Z의위치가-10
  (bind _output_get (Variables|Default|SetZ의%20위치 (+ (Variables|Default|GetZ의%20위치) -1e+01)))
  (Transformation|SetRelativeLocation (Variables|Default|GetCube) (Math|Vector|MakeVector (Variables|Default|GetX의%20위치) 0.0 _output_get) false false))

(fn DoPlayandStop
  (params (IsPlay :type Boolean))
  (Variables|Default|SetIsPlay IsPlay)
  (return false))