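; Actor that slides its Cube component back and forth, as a left-right mover that can be started and stopped.
; A timeline's vector track, scaled mostly along X, sets the Cube's relative location on each update.
; On finish it flips IsRight and re-runs the play/reverse branch, looping endlessly until stopped.
; DoPlayAndStop maps a boolean to the Doplay and DoStop events and always returns false.
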(event Custom|DoStop
  (bind _vector (Timeline|타임라인 Stop)
    (:Update
      (Transformation|SetRelativeLocation (Variables|Default|GetCube) (* _vector "500.000000,10.000000,0.000000") false false))
    (:Finished
      (Variables|Default|SetIsRight (not (Variables|Default|GetIsRight)))
      (if (Variables|Default|GetIsRight)
        (Timeline|타임라인 Play)
        (else
          (Timeline|타임라인 Reverse))))))

(event Custom|Doplay
  (if (Variables|Default|GetIsRight) :!label _label
    (bind _vector (Timeline|타임라인 Play)
      (:Update
        (Transformation|SetRelativeLocation (Variables|Default|GetCube) (* _vector "500.000000,10.000000,0.000000") false false))
      (:Finished
        (Variables|Default|SetIsRight (not (Variables|Default|GetIsRight)))
        (goto _label)))
    (else
      (Timeline|타임라인 Reverse))))

(fn ConstructionScript)

(fn DoPlayandStop
  (params (IsPlay :type Boolean))
  (if IsPlay
    (CallFunction|Doplay)
    (else
      (CallFunction|DoStop)))
  (return false))