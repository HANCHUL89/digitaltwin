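; BP_Timer is a stopwatch Blueprint that displays elapsed minutes and seconds on a TextRender.
; While IsPlay is true, Tick adds delta time to a running total and rewrites the text.
; FloatToStr00 floors each value and zero-pads it to two digits for the MM:SS display.
; DoPlayAndStop sets IsPlay to start or pause counting, with no reset of the total.
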(event EventTick
  (params (DeltaSeconds :type Float%20%28single-precision%29))
  (if (Variables|Default|GetIsPlay)
    (bind _output_get (Variables|Default|SetTotalDeltaSeconds (+ (Variables|Default|GetTotalDeltaSeconds) DeltaSeconds)))
    (Rendering|Components|TextRender|SetText (Variables|Default|GetTextRender) (Utilities|Text|ToText(String) (Utilities|String|Append (Utilities|String|ToString(Text) (Utilities|Text|ToText(String) (CallFunction|FloattoStr00 (/ _output_get 6e+01)))) ":" (Utilities|String|ToString(Text) (Utilities|Text|ToText(String) (CallFunction|FloattoStr00 (Math|Float|%(Float) _output_get 6e+01)))))))))

(fn ConstructionScript)

(fn FloattoStr00
  (params (Number :type Float%20%28double-precision%29))
  (bind _returnvalue (Math|Float|Floor Number))
  (bind _returnvalue_2 (Utilities|String|ToString(Integer) _returnvalue))
  (if (> 10 _returnvalue)
    (return (Utilities|String|Append "0" _returnvalue_2))
    (else
      (return _returnvalue_2))))

(fn DoPlayandStop
  (params (IsPlay :type Boolean))
  (Variables|Default|SetIsPlay IsPlay)
  (return false))