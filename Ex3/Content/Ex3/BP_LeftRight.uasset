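; BP_LeftRight is an actor that slides its Cube component back and forth along the relative X axis.
; While IsPlay is true, Tick steps the X position by a fixed amount per frame, independent of delta time, through two helper functions.
; A direction flag (오른쪽이동인가, "moving right") flips at each end of the range.
; DoPlayAndStop sets IsPlay to start or stop the motion.
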(event EventTick
  (params (DeltaSeconds :type Float%20%28single-precision%29))
  (if (Variables|Default|GetIsPlay)
    (if (Variables|Default|Get오른쪽%20이동인가?)
      (CallFunction|X의위치가+10)
      (if (>= (Variables|Default|GetX의%20위치) 5e+02)
        (Variables|Default|Set오른쪽%20이동인가? false))
      (else
        (CallFunction|X의위치가-10)
        (if (<= (Variables|Default|GetX의%20위치) 0.0)
          (Variables|Default|Set오른쪽%20이동인가? true))))))

(fn ConstructionScript)

(fn X의위치가+10
  (bind _output_get (Variables|Default|SetX의%20위치 (+ (Variables|Default|GetX의%20위치) 1e+01)))
  (Transformation|SetRelativeLocation (Variables|Default|GetCube) (Math|Vector|MakeVector _output_get 0.0 0.0) false false))

(fn X의위치가-10
  (bind _output_get (Variables|Default|SetX의%20위치 (+ (Variables|Default|GetX의%20위치) -1e+01)))
  (Transformation|SetRelativeLocation (Variables|Default|GetCube) (Math|Vector|MakeVector _output_get 0.0 0.0) false false))

(fn DoPlayandStop
  (params (IsPlay :type Boolean))
  (Variables|Default|SetIsPlay IsPlay)
  (return false))