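; BP_Timer3 is an elapsed-time display that shows a running MM:SS clock on a TextRender component.
; Each Tick adds DeltaSeconds to TotalDeltaSeconds, derives minutes by division and seconds by modulo, then updates the text.
; The FloatToStr00 helper floors each value and prepends a zero to single digits.
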(event EventTick
  (params (DeltaSeconds :type Float%20%28single-precision%29))
  (bind _output_get (Variables|Default|SetTotalDeltaSeconds (+ (Variables|Default|GetTotalDeltaSeconds) DeltaSeconds)))
  (bind _str00 (CallFunction|FloattoStr00 (/ _output_get 6e+01)))
  (bind _str00_2 (CallFunction|FloattoStr00 (Math|Float|%(Float) _output_get 6e+01)))
  (Rendering|Components|TextRender|SetText (Variables|Default|GetTextRender) (Utilities|Text|ToText(String) (Utilities|String|Append _str00 ":" _str00_2))))

(fn ConstructionScript)

(fn FloattoStr00
  (params (Number :type Float%20%28double-precision%29))
  (bind _returnvalue (Math|Float|Floor Number))
  (bind _returnvalue_2 (Utilities|String|ToString(Integer) _returnvalue))
  (if (> _returnvalue 9)
    (return _returnvalue_2)
    (else
      (return (Utilities|String|Append "0" _returnvalue_2)))))