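; BP_Timer is a timer that shows elapsed time as MM:SS on a TextRender while running.
; BeginPlay binds to the toggle dispatcher of a referenced Switch, and EventSwitctToggle sets IsPlay from a toggle value to run or pause counting without resetting.
; Tick accumulates time at ten times real speed, and ShowTime formats it with FloatToStr00, which floors and zero-pads each value.
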(event EventTick
  (params (DeltaSeconds :type Float%20%28single-precision%29))
  (if (Variables|Default|GetIsPlay)
    (bind _output_get (Variables|Default|SetTotalDeltaSeconds (+ (Variables|Default|GetTotalDeltaSeconds) (* DeltaSeconds 1e+01))))
    (CallFunction|ShowTime (/ _output_get 6e+01) (Math|Float|%(Float) _output_get 6e+01))))

(event EventBeginPlay
  (EventDispatchers|BindEventtoEventDispatcherToggle (Variables|Default|GetSwitch) (EventDispatchers|CreateEvent :!event EventSwitctToggle)))

(fn ConstructionScript)

(fn FloattoStr00
  (params (Number :type Float%20%28double-precision%29))
  (bind _returnvalue (Math|Float|Floor Number))
  (bind _returnvalue_2 (Utilities|String|ToString(Integer) _returnvalue))
  (if (> _returnvalue 9)
    (return _returnvalue_2 0)
    (else
      (return (Utilities|String|Append "0" _returnvalue_2) 0))))

(fn ShowTime
  (params (Min :type Float%20%28double-precision%29) (Sec :type Float%20%28double-precision%29))
  (Rendering|Components|TextRender|SetText (Variables|Default|GetTextRender) (Utilities|Text|ToText(String) (Utilities|String|Append (.Str00 (CallFunction|FloattoStr00 Min)) ":" (.Str00 (CallFunction|FloattoStr00 Sec))))))

(fn EventSwitctToggle
  (params (Toggle :type Boolean))
  (Variables|Default|SetIsPlay Toggle))