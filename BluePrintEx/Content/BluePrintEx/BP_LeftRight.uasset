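; BP_LeftRight is an example Blueprint whose Cube ping-pongs along its relative X axis while enabled by a switch.
; BeginPlay binds to the referenced Switch's toggle dispatcher, and EventSwitchToggle sets IsPlay from the toggle value.
; While IsPlay is true, Tick calls MoveRight or MoveLeft, flipping IsRight at fixed bounds.
; Movement uses a fixed step per frame without delta time, so speed depends on frame rate.
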(event EventTick
  (params (DeltaSeconds :type Float%20%28single-precision%29))
  (if (Variables|Default|GetIsPlay)
    (if (Variables|Default|GetIsRight)
      (CallFunction|MoveRight)
      (if (>= (Variables|Default|GetPostX) 1e+02)
        (Variables|Default|SetIsRight false))
      (else
        (CallFunction|MoveLeft)
        (if (<= (Variables|Default|GetPostX) 0.0)
          (Variables|Default|SetIsRight true))))))

(event EventBeginPlay
  (EventDispatchers|BindEventtoEventDispatcherToggle (Variables|Default|GetSwitch) (EventDispatchers|CreateEvent :!event EventSwitchToggle)))

(fn ConstructionScript)

(fn MoveRight
  (Variables|Default|SetPostX (+ (Variables|Default|GetPostX) 1e+01))
  (Transformation|SetRelativeLocation (Variables|Default|GetCube) (Math|Vector|MakeVector (Variables|Default|GetPostX) 0.0 0.0) false false))

(fn MoveLeft
  (Variables|Default|SetPostX (+ (Variables|Default|GetPostX) -1e+01))
  (Transformation|SetRelativeLocation (Variables|Default|GetCube) (Math|Vector|MakeVector (Variables|Default|GetPostX) 0.0 0.0) false false))

(fn EventSwitchToggle
  (params (Toggle :type Boolean))
  (Variables|Default|SetIsPlay Toggle))