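; BP_CountBox is an example counter box Blueprint that shows a single-digit count on a TextRender component.
; Each PressF event increments Count, wraps it to zero once it passes nine, updates the text, then calls NewEventDispatcher to notify any listeners.
; Each step is its own small function; leftover Sphere visibility nodes and a Count check are disconnected, and Tick is empty.
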(event EventPressF
  (CallFunction|DoCountUp)
  (CallFunction|Over9Count0)
  (CallFunction|ShowCount)
  (Default|CallNewEventDispatcher))

(event EventTick
  (params (DeltaSeconds :type Float%20%28single-precision%29)))

(fn ConstructionScript)

(fn DoCountUp
  (Variables|Default|SetCount (+ (Variables|Default|GetCount) 1)))

(fn ShowCount
  (Rendering|Components|TextRender|SetText (Variables|Default|GetTextRender) (Utilities|Text|ToText(Integer) (Variables|Default|GetCount))))

(fn Over9Count0
  (if (> (Variables|Default|GetCount) 9)
    (Variables|Default|SetCount 0)))