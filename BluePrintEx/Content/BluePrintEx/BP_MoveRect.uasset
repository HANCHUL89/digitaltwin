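; BP_MoveRect is an actor that moves its Cube component around a square loop in the X-Z plane while switched on.
; On BeginPlay it binds to a Switch object's toggle dispatcher, which appears to set the IsPlay flag via EventSwitchToggle.
; While playing, Tick runs a four-state enum machine that steps the cube's relative location by a fixed, frame-rate-dependent amount, changing direction at each corner.
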(event EventTick
  (params (DeltaSeconds :type Float%20%28single-precision%29))
  (if (Variables|Default|GetIsPlay)
    (switch Utilities|FlowControl|Switch|SwitchonENUM_MoveRect (Variables|Default|GetMoveRect)
      (:NewEnumerator0
        (CallFunction|MoveRight)
        (if (>= (Variables|Default|GetPostX) 1e+02)
          (Variables|Default|SetMoveRect "NewEnumerator1")))
      (:NewEnumerator1
        (CallFunction|MoveUP)
        (if (>= (Variables|Default|GetPostZ) 1e+02)
          (Variables|Default|SetMoveRect "NewEnumerator2")))
      (:NewEnumerator2
        (CallFunction|MoveLeft)
        (if (<= (Variables|Default|GetPostX) 0.0)
          (Variables|Default|SetMoveRect "NewEnumerator3")))
      (:NewEnumerator3
        (CallFunction|MoveDown)
        (if (<= (Variables|Default|GetPostZ) 0.0)
          (Variables|Default|SetMoveRect "NewEnumerator0"))))))

(event EventBeginPlay
  (EventDispatchers|BindEventtoEventDispatcherToggle (Variables|Default|GetSwitch) (EventDispatchers|CreateEvent :!event EventSwitchToggle)))

(fn ConstructionScript)

(fn MoveRight
  (bind _output_get (Variables|Default|SetPostX (+ (Variables|Default|GetPostX) 1e+01)))
  (Transformation|SetRelativeLocation (Variables|Default|GetCube) (Math|Vector|MakeVector _output_get 0.0 (Variables|Default|GetPostZ)) false false))

(fn MoveUP
  (bind _output_get (Variables|Default|SetPostZ (+ (Variables|Default|GetPostZ) 1e+01)))
  (Transformation|SetRelativeLocation (Variables|Default|GetCube) (Math|Vector|MakeVector (Variables|Default|GetPostX) 0.0 _output_get) false false))

(fn MoveLeft
  (bind _output_get (Variables|Default|SetPostX (- (Variables|Default|GetPostX) 1e+01)))
  (Transformation|SetRelativeLocation (Variables|Default|GetCube) (Math|Vector|MakeVector _output_get 0.0 (Variables|Default|GetPostZ)) false false))

(fn MoveDown
  (bind _output_get (Variables|Default|SetPostZ (- (Variables|Default|GetPostZ) 1e+01)))
  (Transformation|SetRelativeLocation (Variables|Default|GetCube) (Math|Vector|MakeVector (Variables|Default|GetPostX) 0.0 _output_get) false false))

(fn EventSwitchToggle
  (params (Toggle :type Boolean))
  (Variables|Default|SetIsPlay Toggle))