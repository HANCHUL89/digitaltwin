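; BP_PortalPassword is a combination lock that toggles a Sphere's visibility based on the counts of a set of CountBox actors.
; BeginPlay hides the Sphere and binds an event to each box's dispatcher.
; FuncPressFClick and 369 show the Sphere only when every box's Count matches the Password entry at its index, using duplicate check functions.
; An order-independent 3-6-9 check, Password369, remains unused.
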(event EventBeginPlay
  (Rendering|SetVisibility (Variables|Default|GetSphere) false false)
  ;[0.15 0.15 0.15 0.5] Count 박스 이벤트 바인딩
  (for _array_element (Variables|Default|GetCountBox)
    (EventDispatchers|BindEventtoNewEventDispatcher _array_element (EventDispatchers|CreateEvent :!event 369))))

(fn ConstructionScript)

(fn IsAllBox9
  (for (_array_element _array_index) (Variables|Default|GetCountBox)
    (if (not (== (Variables|/Game/BluePrintEx/BP_CountBox.BP_CountBox_C|GetCount _array_element) (Utilities|Array|Get(acopy) (Variables|Default|GetPassword) _array_index)))
      (return false)))
  (return true))

(fn FuncPressFClick
  (Development|PrintString "FuncPressFClick")
  (Rendering|SetVisibility (Variables|Default|GetSphere) (CallFunction|IsAllBox9) false))

(fn Password369
  (for _array_element (Variables|Default|GetCountBox)
    (if (== (Variables|/Game/BluePrintEx/BP_CountBox.BP_CountBox_C|GetCount _array_element) 3)
      (for _array_element_2 (Variables|Default|GetCountBox)
        (if (== (Variables|/Game/BluePrintEx/BP_CountBox.BP_CountBox_C|GetCount _array_element_2) 6)
          (for _array_element_3 (Variables|Default|GetCountBox)
            (if (== (Variables|/Game/BluePrintEx/BP_CountBox.BP_CountBox_C|GetCount _array_element_3) 9)
              (return true)))
          (return false))))))

(fn 369
  (Development|PrintString "369")
  (Rendering|SetVisibility (Variables|Default|GetSphere) (CallFunction|Password3692) false))

(fn Password3692
  (for (_array_element _array_index) (Variables|Default|GetCountBox)
    (if (not (== (Variables|/Game/BluePrintEx/BP_CountBox.BP_CountBox_C|GetCount _array_element) (Utilities|Array|Get(acopy) (Variables|Default|GetPassword) _array_index)))
      (return false)))
  (return true))